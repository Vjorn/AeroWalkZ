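; Player attack hitbox actor that detects and applies hits on AI characters while active.
; Each tick it sphere-sweeps from its previous to current location so fast swings register between frames.
; Invincible, same-team and already-hit targets are skipped via the owner's hit list.
; Valid hits scale damage, hitstop and shake by charge and trigger state, then feed GetHit, both hitstop timers, camera shake, meter, style and impact effects.
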(event `Activate`
  (params (Active :type Boolean))
  (bind _output_get (set `self.Active` Active))
  (`self.SetActorHiddenInGame` (not _output_get))
  (`SceneComponent.SetHiddenInGame` (`self.Hitbox`) (not (`/Game/Main/BP_AWGameModeBase.ShowHitboxes` (`/Game/Main/Player/BP_ZPlayerCharacter.GameModeRef` (`self.OwnerCharacter`)))) false)
  (set `self.PreviousLocation` (`self.K2_GetActorLocation`)))

(event `self.ReceiveTick`
  (params (DeltaSeconds :type "Float (single-precision)"))
  (bind _returnvalue (`self.K2_GetActorLocation`))
  (bind _previouslocation (`self.PreviousLocation`))
  (bind _hitdata (`self.HitData`))
  (bind _ownercharacter (`self.OwnerCharacter`))
  (bind ((`Damage_8_265852A247CB84ABE44746ADD5524B74` _damage) (`HitStop_14_7E81BE2A45CDEC159544B58384A4FBD6` _hitstop) (`ShakeScale_16_7984E2C74EF4EA83E0805F9A89611D5C` _shakescale)) (break `/Game/Main/Player/Structs/Struct_HitData` _hitdata))
  (bind ((`Damage_8_265852A247CB84ABE44746ADD5524B74` _damage_2) (`HitStop_14_7E81BE2A45CDEC159544B58384A4FBD6` _hitstop_2) (`ShakeScale_16_7984E2C74EF4EA83E0805F9A89611D5C` _shakescale_2) (`MeterGain_18_5A71B09249B8BC5EBAB55EBFAD0B1DA6` _metergain)) (break `/Game/Main/Player/Structs/Struct_HitData` (`self.ModifiedHitData`)))
  (bind _recentplayermoves (`/Game/Main/Player/BP_ZPlayerController.RecentPlayerMoves` (`/Game/Main/Player/BP_ZPlayerCharacter.PlayerControllerRef` (`self.OwnerCharacter`))))
  (bind _returnvalue_2 (* (select `bool` (or (>= (`ZPlayerCharacter.MeleeChargeLevel` _ownercharacter) 1) (>= (`ZPlayerCharacter.SpecialChargeLevel` _ownercharacter) 1)) :`false` 1.0 :`true` 2.0 :!type "Float (single-precision)") (select `bool` (`ZPlayerCharacter.bTriggerActive` _ownercharacter) :`false` 1.0 :`true` 1.2 :!type "Float (single-precision)")))
  (if (`self.Active`)
    (bind (_outhits _returnvalue_3) (`KismetSystemLibrary.SphereTraceMultiForObjects` (select `bool` (== _previouslocation _returnvalue) :`false` _previouslocation :`true` (+ _previouslocation (0.0 0.0 0.01))) _returnvalue (`SphereComponent.GetScaledSphereRadius` (`self.Hitbox`)) (`|MakeArray` "ObjectTypeQuery8" :!type "EObjectTypeQuery Enum") false (`|MakeArray` (`self.OwnerCharacter`) :!type "Actor Object Reference") "None" true (struct :`R` 1.0 :`A` 1.0) (struct :`G` 1.0 :`A` 1.0) 2.0))
    (set `self.PreviousLocation` (`self.K2_GetActorLocation`))
    (if _returnvalue_3
      (for _array_element _outhits
        (bind (_bblockinghit _binitialoverlap _time _distance _location _impactpoint _normal _impactnormal _physmat _hitactor) (`GameplayStatics.BreakHitResult` _array_element))
        (bind _asbp_z_aibase_character (cast `/Game/Main/AI/Base/BP_Z_AIBaseCharacter` _hitactor))
        (if (not (or (`Z_AIBaseCharacter.bInvincible` _asbp_z_aibase_character) (`KismetArrayLibrary.Array_Contains` (`/Game/Main/Player/BP_ZPlayerCharacter.HitCharacters` (`self.OwnerCharacter`)) _asbp_z_aibase_character) (== (`/Game/Main/AI/Base/BP_Z_AIBaseCharacter.Team` _asbp_z_aibase_character) (`ZPlayerCharacter.Team` (`self.OwnerCharacter`)))))
          (`KismetArrayLibrary.Array_AddUnique` (`/Game/Main/Player/BP_ZPlayerCharacter.HitCharacters` (`self.OwnerCharacter`)) _asbp_z_aibase_character)
          (bind _output_get (set `self.ModifiedHitData` _hitdata))
          (setmembers `/Game/Main/Player/Structs/Struct_HitData` :`StructRef` _output_get :`Damage` (* _damage _returnvalue_2) :`HitStop` (* _hitstop _returnvalue_2) :`ShakeScale` (* _shakescale _returnvalue_2))
          (`/Game/Main/AI/Base/BP_Z_AIBaseCharacter.GetHit` _asbp_z_aibase_character (`self.ModifiedHitData`) self _array_element)
          (set `ZPlayerCharacter.HitstopTime` _hitstop_2 (`self.OwnerCharacter`))
          (set `Z_AIBaseCharacter.HitstopTime` _hitstop_2 _asbp_z_aibase_character)
          (`PlayerCameraManager.PlayCameraShake` :`self` (`GameplayStatics.GetPlayerCameraManager` 0) :`Scale` _shakescale_2)
          (`ZPlayerCharacter.AddMeter` (`self.OwnerCharacter`) _metergain)
          (`/Game/Main/Player/BP_ZPlayerCharacter.AddStyle` (`self.OwnerCharacter`) (`|GetArrayItem` _recentplayermoves (`KismetArrayLibrary.Array_LastIndex` _recentplayermoves)) _damage_2)
          (`/Game/Main/Player/BP_ZPlayerCharacter.HitDetected` (`self.OwnerCharacter`) _array_element)
          (`GameplayStatics.SpawnEmitterAtLocation` null _impactpoint))))))

(fn `UserConstructionScript`)
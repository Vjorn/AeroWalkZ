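; Player camera actor that registers with the game mode, becomes the view target and follows the player character with lock-on support.
; Each tick it interpolates location, spring arm length and rotation.
; While locked on, its pivot blends between player and target by their camera-space depth difference, and zoom grows as the player drifts off the view axis, weighting vertical offset double.
; Otherwise it follows the player at default arm length with clamped pitch.
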(event `self.ReceiveTick`
  (params (DeltaSeconds :type "Float (single-precision)"))
  ;[1 1 1] Tick
  (`self.SetLocation`)
  (`self.SetZoom`)
  (`self.SetRotation`))

(event `self.ReceiveBeginPlay`
  ;[1 1 1] Initialize
  (bind _asbp_awgame_mode_base (cast `/Game/Main/BP_AWGameModeBase` (`GameplayStatics.GetGameMode`)))
  (bind _output_get (set `self.ZGameMode` _asbp_awgame_mode_base))
  (bind _output_get_2 (set `/Game/Main/BP_AWGameModeBase.ZPlayerCamera` self _output_get))
  (`PlayerController.SetViewTargetWithBlend` (`GameplayStatics.GetPlayerController` 0) _output_get_2 0.0 "VTBlend_Linear" 0.0 false)
  (bind _asbp_zplayer_character (cast `/Game/Main/Player/BP_ZPlayerCharacter` (`GameplayStatics.GetPlayerCharacter` 0)))
  (set `self.ZPlayer` _asbp_zplayer_character))

(event `SetLocation`
  (bind _zplayer (`self.ZPlayer`))
  (bind _returnvalue (`self.K2_GetActorLocation` (`self.ZPlayer`)))
  (bind _returnvalue_2 (`SceneComponent.K2_GetComponentRotation` (`self.Camera`)))
  (bind _returnvalue_3 (`self.K2_GetActorLocation` (`/Game/Main/Player/BP_ZPlayerCharacter.LockOnTarget` (`self.ZPlayer`))))
  ;[1 1 1] Update camera location
  (`/Engine/EditorBlueprintResources/StandardMacros.IsValid` _zplayer
    (:`Is Valid`
      (if (`ZPlayerCharacter.bIsLockedOn` _zplayer)
        (`self.K2_SetActorLocation` (`KismetMathLibrary.VInterpTo` (`self.K2_GetActorLocation`) (`KismetMathLibrary.VLerp` _returnvalue _returnvalue_3 (`KismetMathLibrary.MapRangeClamped` (- (.x (`KismetMathLibrary.LessLess_VectorRotator` _returnvalue _returnvalue_2)) (.x (`KismetMathLibrary.LessLess_VectorRotator` _returnvalue_3 _returnvalue_2))) -5000.0 5000.0 0.0 1.0)) (`GameplayStatics.GetWorldDeltaSeconds`) (* (`self.LockOnInterpSpeed`) 3.0)))
        (else
          (`self.K2_SetActorLocation` (`KismetMathLibrary.VInterpTo` (`self.K2_GetActorLocation`) (`self.K2_GetActorLocation` _zplayer) (`GameplayStatics.GetWorldDeltaSeconds`) (* (`self.UnlockInterpSpeed`) 1.5))))))))

(event `SetZoom`
  (bind _camera (`self.Camera`))
  ;[1 1 1] Update camera zoom
  (if (`ZPlayerCharacter.bIsLockedOn` (`self.ZPlayer`))
    (set `SpringArmComponent.TargetArmLength` (`KismetMathLibrary.FInterpTo` (`SpringArmComponent.TargetArmLength` (`self.SpringArm`)) (+ (* (- 1.0 (`KismetMathLibrary.Dot_VectorVector` (1.0 0.0 0.0) (`KismetMathLibrary.Normal` (* (`KismetMathLibrary.LessLess_VectorRotator` (`KismetMathLibrary.GetDirectionUnitVector` (`SceneComponent.K2_GetComponentLocation` _camera) (`self.K2_GetActorLocation` (`self.ZPlayer`))) (`SceneComponent.K2_GetComponentRotation` _camera)) (1.0 1.0 2.0))))) 2500.0) (`self.LockOnArmLengthOffset`)) (`GameplayStatics.GetWorldDeltaSeconds`) (`self.LockOnInterpSpeed`)) (`self.SpringArm`))
    (else
      (set `SpringArmComponent.TargetArmLength` (`KismetMathLibrary.FInterpTo` (`SpringArmComponent.TargetArmLength` (`self.SpringArm`)) (`self.DefaultArmLength`) (`GameplayStatics.GetWorldDeltaSeconds`) (`self.UnlockInterpSpeed`)) (`self.SpringArm`)))))

(event `SetRotation`
  (bind _returnvalue (`self.K2_GetActorRotation`))
  ;[1 1 1] Update camera rotation
  (if (not (`ZPlayerCharacter.bIsLockedOn` (`self.ZPlayer`)))
    (`self.K2_SetActorRotation` (`KismetMathLibrary.RInterpTo` _returnvalue (`KismetMathLibrary.MakeRotator` 0.0 (`KismetMathLibrary.FClamp` (.pitch _returnvalue) -60.0 60.0) (.yaw _returnvalue)) (`GameplayStatics.GetWorldDeltaSeconds`) 30.0))))

(fn `UserConstructionScript`)
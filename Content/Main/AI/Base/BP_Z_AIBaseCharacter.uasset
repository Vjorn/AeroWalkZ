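; Base AI combat character that handles hit reactions, damage, landing and movement recovery.
; GetHit launches it by the hit data, plays air or ground hitstun, and subtracts health if the game mode allows, calling an empty Die at zero.
; Tick detects landings and eases gravity and friction back to targets.
; Hurtboxes follow skeleton sockets; repulsion events, not called here, average sphere overlaps with players and enemies into a push-apart offset.
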(event `self.ReceiveTick`
  (params (DeltaSeconds :type "Float (single-precision)"))
  (`self.LandCheck`)
  (`self.InterpMovement`))

(event `self.ReceiveBeginPlay`
  (bind _asbp_awgame_mode_base (cast `/Game/Main/BP_AWGameModeBase` (`GameplayStatics.GetGameMode`)))
  (set `self.ZGameModeRef` _asbp_awgame_mode_base)
  (set `self.RepelSpheres` (`|MakeArray` (`self.RepelSphere`))))

(event `StartAnim`
  (set `self.FloatTime` 0.0)
  (`self.ClearHitboxes`)
  (`KismetArrayLibrary.Array_Clear` (`self.HitCharacters`))
  (set `self.bPhaseThrough` false)
  (set `self.bGuarding` false)
  (set `self.GuardTime` 0.0)
  (set `self.bCollisionStop` false)
  (set `self.JumpTimer` 0.0)
  (`self.SetInvinciblity` false)
  (set `self.bCombatAnimation` true)
  (set `self.bMeleeCharge` false)
  (set `self.bSpecialCharge` false)
  (set `self.MeleeChargeLevel` -1)
  (set `self.SpecialChargeLevel` -1))

(event `ClearHitboxes`
  (for _array_element (`self.Hitboxes`)
    (`/Game/Main/Player/BP_ZHitbox.Activate` _array_element false))
  (`KismetArrayLibrary.Array_Clear` (`self.HitCharacters`)))

(event `SetInvinciblity`
  (params (Invincible :type Boolean))
  (bind _output_get (set `self.bInvincible` Invincible))
  (for _array_element (`self.Hurtboxes`)
    (`PrimitiveComponent.SetCollisionEnabled` _array_element (select `bool` _output_get :`false` "QueryOnly" :`true` "NoCollision" :!type "ECollisionEnabled Enum"))))

(event `GetHit`
  (params (HitData :type "/Game/Main/Player/Structs/Struct_HitData Structure") (AttackerHitbox :type "/Game/Main/Player/BP_ZHitbox Object Reference") (HitResult :type "HitResult Structure"))
  (bind (_directiontype _launchvector _damage _launchtype) (break `/Game/Main/Player/Structs/Struct_HitData` HitData))
  (bind _charactermovement (`self.CharacterMovement`))
  (bind _ownercharacter (`/Game/Main/Player/BP_ZHitbox.OwnerCharacter` AttackerHitbox))
  (bind _returnvalue (`KismetMathLibrary.GreaterGreater_VectorRotator` _launchvector (`KismetMathLibrary.MakeRotator` 0.0 0.0 (.yaw (select `int` _directiontype :`0` (`KismetMathLibrary.FindLookAtRotation` (`self.K2_GetActorLocation` _ownercharacter) (`self.K2_GetActorLocation`)) :`1` (`self.K2_GetActorRotation` _ownercharacter))))))
  (`KismetSystemLibrary.PrintString` "AI_GetHit")
  (`Controller.StopMovement` (`self.GetController`))
  (bind _output_get (set `MovementComponent.Velocity` (select `int` _launchtype :`0` (0.0 0.0 0.0) :`1` (select `bool` (`self.bInAir`) :`false` (`KismetMathLibrary.Conv_Vector2DToVector` (`KismetMathLibrary.Conv_VectorToVector2D` _returnvalue)) :`true` _returnvalue) :`2` _returnvalue) (`self.CharacterMovement`)))
  (`self.RestoreMovementDefaults` false)
  (`self.K2_SetActorRotation` (select `int` 0 :`0` (`KismetMathLibrary.MakeRotator` 0.0 0.0 (.yaw (`KismetMathLibrary.FindLookAtRotation` (`self.K2_GetActorLocation`) (`self.K2_GetActorLocation` _ownercharacter)))) :`1` (`KismetMathLibrary.MakeRotator` 0.0 0.0 (.yaw (`KismetMathLibrary.MakeRotFromX` (* (`self.GetActorForwardVector` _ownercharacter) -1.0))))))
  (if (!= (.z _output_get) 0.0)
    (set `self.bInAir` true)
    (`CharacterMovementComponent.SetMovementMode` _charactermovement "MOVE_Falling" 0)
    (set `CharacterMovementComponent.GravityScale` 0.0 _charactermovement))
  (`self.HurtAnimation` AttackerHitbox)
  (`self.TakeDamage` _damage))

(event `Die`)

(event `TakeDamage`
  (params (Damage :type "Float (double-precision)"))
  (if (`/Game/Main/BP_AWGameModeBase.EnableDamage` (`self.ZGameModeRef`))
    (bind _output_get (set `self.Health` (`KismetMathLibrary.FClamp` (- (`self.Health`) Damage) 0.0 (`self.MaxHealth`))))
    (if (<= _output_get 0.0)
      (`self.Die`))))

(event `HurtAnimation`
  (params (AttackerHitbox :type "/Game/Main/Player/BP_ZHitbox Object Reference"))
  (bind _ownercharacter (`/Game/Main/Player/BP_ZHitbox.OwnerCharacter` AttackerHitbox))
  (if (`self.bInAir`)
    (`self.PlayAnimMontage` "/Game/Main/AI/Base/AnimMontages/Base_Hitstun_Air_Montage.Base_Hitstun_Air_Montage" 1.0 "None")
    (else
      (`self.PlayAnimMontage` (select `bool` (or (>= (`ZPlayerCharacter.MeleeChargeLevel` _ownercharacter) 1) (>= (`ZPlayerCharacter.SpecialChargeLevel` _ownercharacter) 1)) :`false` "/Game/Main/AI/Base/AnimMontages/Base_Hitstun_Montage.Base_Hitstun_Montage" :`true` "/Game/Main/AI/Base/AnimMontages/Base_Hitstun_Long_Montage.Base_Hitstun_Long_Montage" :!type "AnimMontage Object Reference") 1.0 "None")))
  (`self.StartAnim`)
  (`self.CanDo` false true)
  (set `self.bCanEnemyStep` false)
  (set `self.StateIndex` 4))

(event `CalculateCharacterRepulsion`
  (bind _repelenemies (`self.RepelEnemies`))
  (bind _repelplayer (`self.RepelPlayer`))
  (`KismetArrayLibrary.Array_Clear` (`self.RepelVectors`))
  (`KismetArrayLibrary.Array_Clear` (`self.RepelEnemies`))
  (`KismetArrayLibrary.Array_Clear` (`self.RepelPlayer`))
  (`KismetArrayLibrary.Array_Clear` (`self.RepelVectors`))
  (if (not (`self.bPhaseThrough`))
    (for _array_element (`self.RepelSpheres`)
      (`|ExecutionSequence`
        (:`then_0`
          (for _array_element_2 (`/Game/Main/BP_AWGameModeBase.Players` (`self.ZGameModeRef`))
            (if (not (`ZPlayerCharacter.bPhaseThrough` _array_element_2))
              (for _array_element_3 (`/Game/Main/Player/BP_ZPlayerCharacter.RepelSpheres` _array_element_2)
                (bind _returnvalue (`SceneComponent.K2_GetComponentLocation` _array_element_3))
                (bind _returnvalue_2 (`SceneComponent.K2_GetComponentLocation` _array_element))
                (bind _returnvalue_3 (`KismetMathLibrary.Vector_Distance` _returnvalue _returnvalue_2))
                (bind _returnvalue_4 (`SphereComponent.GetScaledSphereRadius` _array_element_3))
                (bind _returnvalue_5 (`SphereComponent.GetScaledSphereRadius` _array_element))
                (bind _returnvalue_6 (+ (`KismetMathLibrary.FClamp` (- _returnvalue_4 1.0) 0.0 _returnvalue_4) (`KismetMathLibrary.FClamp` (- _returnvalue_5 1.0) 0.0 _returnvalue_5)))
                (if (< _returnvalue_3 _returnvalue_6)
                  (if (`KismetArrayLibrary.Array_Contains` _repelplayer _array_element_2)
                    (bind _returnvalue_7 (- _returnvalue_6 _returnvalue_3))
                    (bind _returnvalue_8 (`KismetArrayLibrary.Array_Find` (`self.RepelPlayer`) _array_element_2))
                    (if (> _returnvalue_7 (`KismetMathLibrary.VSize` (`|GetArrayItem` (`self.RepelVectors`) _returnvalue_8)))
                      (bind _returnvalue_9 (* (`KismetMathLibrary.Vector_Normal2D` (`KismetMathLibrary.GetDirectionUnitVector` _returnvalue _returnvalue_2)) _returnvalue_7))
                      (`KismetArrayLibrary.Array_Set` (`self.RepelVectors`) _returnvalue_8 _returnvalue_9 true))
                    (else
                      (`KismetArrayLibrary.Array_Add` _repelplayer)
                      (`KismetArrayLibrary.Array_Add` (`self.RepelVectors`) _returnvalue_9))))))))
        (:`then_1`
          (for _array_element_4 (`/Game/Main/BP_AWGameModeBase.Enemies` (`self.ZGameModeRef`))
            (if (not (`Z_AIBaseCharacter.bPhaseThrough` _array_element_4))
              (for _array_element_5 (`/Game/Main/AI/Base/BP_Z_AIBaseCharacter.RepelSpheres` _array_element_4)
                (bind _returnvalue_10 (`SceneComponent.K2_GetComponentLocation` _array_element_5))
                (bind _returnvalue_11 (`SceneComponent.K2_GetComponentLocation` _array_element))
                (bind _returnvalue_12 (`KismetMathLibrary.Vector_Distance` _returnvalue_10 _returnvalue_11))
                (bind _returnvalue_13 (`SphereComponent.GetScaledSphereRadius` _array_element_5))
                (bind _returnvalue_14 (`SphereComponent.GetScaledSphereRadius` _array_element))
                (bind _returnvalue_15 (+ (`KismetMathLibrary.FClamp` (- _returnvalue_13 1.0) 0.0 _returnvalue_13) (`KismetMathLibrary.FClamp` (- _returnvalue_14 1.0) 0.0 _returnvalue_14)))
                (if (< _returnvalue_12 _returnvalue_15)
                  (if (`KismetArrayLibrary.Array_Contains` _repelenemies _array_element_4)
                    (bind _returnvalue_16 (- _returnvalue_15 _returnvalue_12))
                    (bind _returnvalue_17 (`KismetArrayLibrary.Array_Find` (`self.RepelEnemies`) _array_element_4))
                    (if (> _returnvalue_16 (`KismetMathLibrary.VSize` (`|GetArrayItem` (`self.RepelVectors`) _returnvalue_17)))
                      (bind _returnvalue_18 (* (`KismetMathLibrary.Vector_Normal2D` (`KismetMathLibrary.GetDirectionUnitVector` _returnvalue_10 _returnvalue_11)) _returnvalue_16))
                      (`KismetArrayLibrary.Array_Set` (`self.RepelVectors`) _returnvalue_17 _returnvalue_18 true))
                    (else
                      (`KismetArrayLibrary.Array_Add` _repelenemies)
                      (`KismetArrayLibrary.Array_Add` (`self.RepelVectors`) _returnvalue_18))))))))))))

(event `CharacterRepulsion`
  (`self.K2_AddActorWorldOffset` (/ (`KismetMathLibrary.GetVectorArrayAverage` (`self.RepelVectors`)) 2.0) true))

(event `InterpMovement`
  (bind _charactermovement (`self.CharacterMovement`))
  (bind _charactermovement_2 (`self.CharacterMovement`))
  (bind _floattime (`self.FloatTime`))
  (bind _floattime_2 (`self.FloatTime`))
  (if (== _floattime_2 0.0)
    (set `CharacterMovementComponent.GravityScale` (`KismetMathLibrary.FInterpTo` (`CharacterMovementComponent.GravityScale` (`self.CharacterMovement`)) (`self.TargetGravity`) (* (`GameplayStatics.GetWorldDeltaSeconds`) (`self.CustomTimeDilation`)) 5.0) (`self.CharacterMovement`))
    (elif (> _floattime_2 0.0)
      (set `self.FloatTime` (`KismetMathLibrary.FClamp` (- _floattime (* (`GameplayStatics.GetWorldDeltaSeconds`) (`self.CustomTimeDilation`))) 0.0 _floattime))))
  (set `CharacterMovementComponent.GroundFriction` (`KismetMathLibrary.FInterpTo` (`CharacterMovementComponent.GroundFriction` _charactermovement) (`self.TargetGroundFriction`) (* (`GameplayStatics.GetWorldDeltaSeconds`) (`self.CustomTimeDilation`)) 5.0) _charactermovement)
  (set `CharacterMovementComponent.FallingLateralFriction` (`KismetMathLibrary.FInterpTo` (`CharacterMovementComponent.FallingLateralFriction` _charactermovement_2) (`self.TargetAirFriction`) (* (`GameplayStatics.GetWorldDeltaSeconds`) (`self.CustomTimeDilation`)) 5.0) _charactermovement_2))

(event `LandCheck`
  (bind _returnvalue (`NavMovementComponent.IsFalling` (`self.CharacterMovement`)))
  (if _returnvalue
    (set `self.bInAir` _returnvalue)
    (elif (`self.bInAir`)
      (`self.ForceLand`))))

(event `ForceLand`
  (set `self.bInAir` false :!label _label)
  (if (== (`self.StateIndex`) 4)
    (`self.PlayAnimMontage` "/Game/Main/AI/Base/AnimMontages/Base_Hitstun_air_land_Montage.Base_Hitstun_air_land_Montage" 1.0 "None")
    (`self.RestoreMovementDefaults` false)
    (set `self.bCombatAnimation` true)
    (elif (== (`self.StateIndex`) 5)
      (`self.PlayAnimMontage` "/Game/Main/AI/Base/AnimMontages/Base_Hitstun_Air_HardKnockdown_Land_Montage.Base_Hitstun_Air_HardKnockdown_Land_Montage" 1.0 "None")
      (else
        (`self.PlayAnimMontage` "/Game/Main/AI/Base/AnimMontages/Base_Jump_Montage.Base_Jump_Montage" 1.0 "Land")
        (`self.CanDo` true true)
        (`self.StartAnim`)
        (`self.RestoreMovementDefaults` false)
        (set `self.bCombatAnimation` false)))))

(event `self.OnLanded`
  (params (Hit :type "HitResult Structure (by ref)"))
  (goto _label))

(fn `UserConstructionScript`
  (bind _mesh (`self.Mesh`))
  (`SceneComponent.K2_AttachToComponent` (`self.HurtboxTorso`) _mesh "spine_02" "KeepRelative" "KeepRelative" "KeepRelative" true)
  (`SceneComponent.K2_AttachToComponent` (`self.HurtboxLegL`) _mesh "calf_l" "KeepRelative" "KeepRelative" "KeepRelative" true)
  (`SceneComponent.K2_AttachToComponent` (`self.HurtboxLegR`) _mesh "calf_r" "KeepRelative" "KeepRelative" "KeepRelative" true)
  (`SceneComponent.K2_AttachToComponent` (`self.RepelSphere`) _mesh "spine_02" "KeepRelative" "KeepRelative" "KeepRelative" true)
  (set `self.Hurtboxes` (`|MakeArray` (`self.HurtboxTorso`) (`self.HurtboxLegL`) (`self.HurtboxLegR`))))